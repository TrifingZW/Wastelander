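; BP_MLRS is an MLRS vehicle Blueprint that drives itself at full throttle once a player interaction starts its engine.
; InteractionTarget is enabled on BeginPlay, and its interaction event sets the Engine flag, then blocks further interaction.
; While the flag is set, Tick feeds full throttle to VehicleMovementComponent every frame.
; The graph has no steering, braking, engine shutoff or weapon logic, and the construction script is empty.
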(event `self.ReceiveTick`
  (params (DeltaSeconds :type "Float (single-precision)"))
  (if (`self.Engine`)
    (`ChaosVehicleMovementComponent.SetThrottleInput` (`self.VehicleMovementComponent`) 1.0)))

(event `self.InteractionTarget.OnInteractionEvent`
  (params (Interactor :type "Actor Object Reference") (Value :type "InputActionValue Structure (by ref)"))
  (set `self.Engine` true)
  (`InteractionTarget.BlockInteraction` (`self.InteractionTarget`)))

(event `self.ReceiveBeginPlay`
  (`InteractionTarget.EnableInteraction` (`self.InteractionTarget`)))

(fn `UserConstructionScript`)